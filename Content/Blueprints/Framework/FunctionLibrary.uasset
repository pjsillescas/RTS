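; Blueprint function library of helpers for grid-based building placement and an in-game clock.
; Cursor positioning line-traces from the deprojected mouse, returning the hit location or zero, and GridSnap rounds a coordinate to the grid.
; SetClockwork advances time by scaled delta seconds, wrapping at 24 and outputting elapsed days.
; Two building helpers use mesh local bounds to position an entrance component and size and place a collision box.
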(fn SetCursorWorldPosition
  (params (Controller :type BP%20Camera%20Pawn%20Controller%20Object%20Reference) (SightDistance :type Float%20%28single-precision%29))
  (bind (_worldlocation _worlddirection) (Game|Player|ConvertMouseLocationToWorldSpace Controller))
  (bind _outhit (Collision|LineTraceByChannel 0 _worldlocation (+ _worldlocation (* _worlddirection SightDistance)) "TraceTypeQuery3" false 0 "None"))
  (Utilities|IsValid (.HitActor (Collision|BreakHitResult _outhit))
    (:Is%20Valid
      (return (.Location (Collision|BreakHitResult _outhit))))
    (:Is%20Not%20Valid
      (return "0, 0, 0"))))

(fn GridSnap
  (params (Axis :type Float%20%28single-precision%29) (GridSize :type Integer))
  (return (Math|Conversions|ToFloat(Integer) (* (Math|Float|Floor (/ (+ Axis (Math|Conversions|ToFloat(Integer) (/ GridSize 2))) (Math|Conversions|ToFloat(Integer) GridSize))) GridSize))))

(fn SetClockwork
  (params (DeltaSeconds :type Float%20%28single-precision%29) (TimeUnit :type Float%20%28single-precision%29) (ClockworkIn :type Float%20%28single-precision%29))
  (bind _returnvalue (/ DeltaSeconds TimeUnit))
  (bind _returnvalue_2 (+ _returnvalue ClockworkIn))
  (bind (_remainder _returnvalue_3) (Math|Float|Division(WholeandRemainder) _returnvalue_2 24.0))
  (return _remainder _returnvalue_3))

(fn SetBuildingCollisionBox
  (params (Collision :type Box%20Component%20Object%20Reference) (Mesh :type Static%20Mesh%20Component%20Object%20Reference))
  (bind _min (Components|StaticMesh|GetLocalBounds Mesh))
  (Components|Box|SetBoxExtent Collision (Math|Vector|MakeVector 49.0 (- (Math|Float|Absolute(Float) (.y _min)) 1e+01) 1e+01) true)
  (Transformation|SetRelativeLocation Collision (Math|Vector|MakeVector (+ (Math|Float|Absolute(Float) (.x _min)) (LocalVariables|GetBoxExtentX)) 0.0 1e+01) false false))

(fn SetBuildingEntrance
  (params (Scene :type Scene%20Component%20Object%20Reference) (Mesh :type Static%20Mesh%20Component%20Object%20Reference))
  (Transformation|SetRelativeLocation Scene (Math|Vector|MakeVector (+ (Math|Float|Absolute(Float) (.x (.Min (Components|StaticMesh|GetLocalBounds Mesh)))) (LocalVariables|GetLEntranceDistance)) 0.0 0.0) false false))