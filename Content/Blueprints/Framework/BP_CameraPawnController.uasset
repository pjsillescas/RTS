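; Player controller for a top-down building game, driving a camera pawn and handling building placement and selection.
; On BeginPlay it spawns the construction manager and ghost building, then creates the main HUD and passes it to the game state.
; Input pans, zooms and moves the camera, including screen-edge scrolling, with key-movement speed scaled by zoom.
; In build mode the ghost tracks the cursor, rotates, and queues construction when not overlapping.
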(event EventBeginPlay
  (Variables|Default|SetbShowMouseCursor true)
  (Input|SetInputModeGameandUI self 0 "DoNotLock" false)
  (Utilities|FlowControl|Sequence
    (:then_0
      (Utilities|ReferenceCasts))
    (:then_1
      (bind _returnvalue (Game|SpawnActorfromClass "/Game/Blueprints/Construction/BP_ConstructionManager.BP_ConstructionManager_C" (Math|Transform|MakeTransform "0, 0, 0" "0, 0, 0" "0.500000,0.500000,0.500000") "Undefined" 0 0))
      (Variables|References|SetConstructionManagerRef _returnvalue)
      (bind _returnvalue_2 (Game|SpawnActorfromClass "/Game/Blueprints/Buildings/BP_GhostBuilding.BP_GhostBuilding_C" (Math|Transform|MakeTransform "0, 0, 0" "0, 0, 0" "0.500000,0.500000,0.500000") "Undefined" 0 self 0))
      (Variables|References|SetGhostBuildingRef _returnvalue_2))
    (:then_2
      (Utilities|CreateHuds)
      (UserInterface|Viewport|AddtoViewport (Variables|References|GetMainHudRef) 0)
      (Default|SetHud (Variables|References|GetGameStateRef) (Variables|References|GetMainHudRef)))))

(event EventTick
  (params (DeltaSeconds :type Float%20%28single-precision%29))
  (if (Variables|Default|GetbBuildModeActive)
    (Utilities|IsValid (Variables|References|GetGhostBuildingRef)
      (:Is%20Valid
        (Variables|/Game/Blueprints/Buildings/BP_GhostBuilding.BP_GhostBuilding_C|SetCursorWorldPosition (Variables|References|GetGhostBuildingRef) (CallFunction|SetCursorWorldPosition self (CallFunction|SetSightDistance)))))))

(event Input|KeyboardEvents|V
  (params (Key :type Key%20Structure))
  (bind _self self)
  (bind _mouselocation (CallFunction|SetCursorWorldPosition _self 1e+04))
  (:Pressed
    (Game|SpawnActorfromClass "/Game/Blueprints/NPC/NPC_BP.NPC_BP_C" (Math|Transform|MakeTransform (Math|Vector|MakeVector (.x _mouselocation) (.y _mouselocation) 92.0) "0, 0, 0" "0.500000,0.500000,0.500000") "Undefined" 0 0)))

(event Custom|ApplyZoom
  (params (Distance :type Float%20%28single-precision%29))
  ;[1 1 1] Zoom In/Out
  (Variables|/Script/Engine.SpringArmComponent|SetTargetArmLength (Variables|/Game/Blueprints/Framework/BP_CameraPawn.BP_CameraPawn_C|GetSpringArm (Variables|References|GetCameraPawnRef)) (Math|Float|Clamp(Float) (+ Distance (Variables|/Script/Engine.SpringArmComponent|GetTargetArmLength (Variables|/Game/Blueprints/Framework/BP_CameraPawn.BP_CameraPawn_C|GetSpringArm (Variables|References|GetCameraPawnRef)))) 1e+03 (Variables|Default|GetMaxArmDistance))))

(event Custom|AddGhostBuildingYaw
  (params (DeltaYaw :type Float%20%28single-precision%29))
  (bind _ghostbuildingref (Variables|References|GetGhostBuildingRef))
  (bind _returnvalue (Transformation|GetActorRotation _ghostbuildingref))
  ;[1 1 1] Building Yaw Change
  (if (and (Utilities|IsValid (Variables|References|GetGhostBuildingRef)) (Variables|Default|GetbBuildModeActive))
    (Transformation|SetActorRotation (Variables|References|GetGhostBuildingRef) (Math|Rotator|MakeRotator (.roll _returnvalue) (.pitch _returnvalue) (+ (.yaw _returnvalue) DeltaYaw)))))

(event Input|ActionEvents|InputActionPan
  (params (Key :type Key%20Structure :default "None"))
  (bind _camerapawnref (Variables|References|GetCameraPawnRef))
  (bind _returnvalue (Transformation|GetActorRotation _camerapawnref))
  ;[1 1 1] Pan Y
  (:Pressed
    (Variables|Default|SetbDisableCamNav true)
    (Utilities|FlowControl|Gate true) ; enters at Open
  )
  (:Released
    (Variables|Default|SetbDisableCamNav false)
    (Utilities|FlowControl|Gate true) ; enters at Close
  ))

(event Input|ActionEvents|InputActionPan
  (params (Key :type Key%20Structure :default "None"))
  (bind _camerapawnref (Variables|References|GetCameraPawnRef))
  (bind _returnvalue (Transformation|GetActorRotation _camerapawnref))
  ;[1 1 1] Pan X
  (:Pressed
    (Variables|Default|SetbDisableCamNav true)
    (Utilities|FlowControl|Gate true) ; enters at Open
  )
  (:Released
    (Variables|Default|SetbDisableCamNav false)
    (Utilities|FlowControl|Gate true) ; enters at Close
  ))

(event Input|ActionEvents|InputActionPanReset
  (params (Key :type Key%20Structure :default "None"))
  (bind _camerapawnref (Variables|References|GetCameraPawnRef))
  (bind _returnvalue (Transformation|GetActorRotation _camerapawnref))
  ;[1 1 1] Pan Reset
  (:Pressed
    (Transformation|SetActorRotation _camerapawnref (Math|Rotator|MakeRotator (.roll _returnvalue) 0.0 (.yaw _returnvalue)))))

(event Input|ActionEvents|InputActionZoomIn
  (params (Key :type Key%20Structure :default "None"))
  ;[1 1 1] Zoom In/Out
  (:Pressed
    (CallFunction|ApplyZoom (* (Variables|Default|GetZoomSensitivity) -1.0))))

(event Input|ActionEvents|InputActionZoomOut
  (params (Key :type Key%20Structure :default "None"))
  ;[1 1 1] Zoom In/Out
  (:Pressed
    (CallFunction|ApplyZoom (Variables|Default|GetZoomSensitivity))))

(event Input|ActionEvents|InputActionZoomReset
  (params (Key :type Key%20Structure :default "None"))
  ;[1 1 1] Zoom Reset
  (:Pressed
    (Variables|/Script/Engine.SpringArmComponent|SetTargetArmLength (Variables|/Game/Blueprints/Framework/BP_CameraPawn.BP_CameraPawn_C|GetSpringArm (Variables|References|GetCameraPawnRef)) 2.5e+03)))

(event Input|ActionEvents|InputActionDeselect
  (params (Key :type Key%20Structure :default "None"))
  ;[1 1 1] Deselect
  (:Pressed
    (if (Variables|Default|GetbBuildModeActive)
      (Default|KillGhost (Variables|References|GetGhostBuildingRef))
      (Variables|Default|SetbBuildModeActive false))))

(event Input|ActionEvents|InputActionRotateBuildingLeft
  (params (Key :type Key%20Structure :default "None"))
  ;[1 1 1] Building Yaw Change
  (:Pressed
    (CallFunction|AddGhostBuildingYaw (* (Variables|Default|GetBuildingRotationRate) -1.0))))

(event Input|ActionEvents|InputActionRotateBuildingRight
  (params (Key :type Key%20Structure :default "None"))
  ;[1 1 1] Building Yaw Change
  (:Pressed
    (CallFunction|AddGhostBuildingYaw (Variables|Default|GetBuildingRotationRate))))

(event Input|AxisEvents|InputAxisMoveForward
  (params (AxisValue :type Float%20%28single-precision%29))
  ;[1 1 1] Movement X
  (if (not (Variables|Default|GetbDisableCamNav))
    (Transformation|SetActorTransform (Variables|References|GetCameraPawnRef) (Utilities|MovementX AxisValue (CallFunction|MovementSpeedCalculation) (Variables|Default|GetFastMoveMultiplier) (Variables|References|GetCameraPawnRef)))))

(event Input|AxisEvents|InputAxisMoveRight
  (params (AxisValue :type Float%20%28single-precision%29))
  (bind _movesensitivity (CallFunction|MovementSpeedCalculation))
  (bind _fastmovemultiplier (Variables|Default|GetFastMoveMultiplier))
  (bind _camerapawnref (Variables|References|GetCameraPawnRef))
  (bind _transform (Utilities|MovementY AxisValue _movesensitivity _fastmovemultiplier _camerapawnref))
  ;[1 1 1] Movement Y
  (if (not (Variables|Default|GetbDisableCamNav))
    (Transformation|SetActorTransform (Variables|References|GetCameraPawnRef) (Math|Transform|MakeTransform (Math|Vector|MakeVector (.x (.location _transform)) (.y (.location _transform)) 0.0) (.rotation _transform) (.scale _transform)))))

(event Input|MouseEvents|MouseX
  (params (AxisValue :type Float%20%28single-precision%29))
  (bind _camerapawnref (Variables|References|GetCameraPawnRef))
  (bind _returnvalue (Transformation|GetActorRotation _camerapawnref))
  ;[1 1 1] Pan X
  (Utilities|FlowControl|Gate true
    (:Exit
      (Transformation|SetActorRotation (Variables|References|GetCameraPawnRef) (Math|Rotator|MakeRotator (.roll _returnvalue) (.pitch _returnvalue) (+ (.yaw _returnvalue) (* AxisValue (Variables|Default|GetPanSensitivity))))))))

(event Input|MouseEvents|MouseY
  (params (AxisValue :type Float%20%28single-precision%29))
  (bind _camerapawnref (Variables|References|GetCameraPawnRef))
  (bind _returnvalue (Transformation|GetActorRotation _camerapawnref))
  ;[1 1 1] Pan Y
  (Utilities|FlowControl|Gate true
    (:Exit
      (Transformation|SetActorRotation (Variables|References|GetCameraPawnRef) (Math|Rotator|MakeRotator (.roll _returnvalue) (Math|Float|Clamp(Float) (+ (.pitch _returnvalue) (* AxisValue (Variables|Default|GetPanSensitivity))) -15.0 45.0) (.yaw _returnvalue))))))

(event Input|MouseEvents|MouseX
  (params (AxisValue :type Float%20%28single-precision%29))
  ;[1 1 1] Edge Movement
  (if (not (Variables|Default|GetbDisableCamNav))
    (bind (_deltaxspeed _deltayspeed) (Utilities|ScreenEdgeMovement))
    (Transformation|AddActorLocalOffset (Variables|References|GetCameraPawnRef) (Math|Vector|MakeVector _deltaxspeed _deltayspeed 0.0) true false)))

(event Input|MouseEvents|MouseY
  (params (AxisValue :type Float%20%28single-precision%29))
  ;[1 1 1] Edge Movement
  (if (not (Variables|Default|GetbDisableCamNav))
    (Utilities|ScreenEdgeMovement) ; enters at MouseY
  ))

(event Input|KeyboardEvents|LeftShift
  (params (Key :type Key%20Structure :default "None"))
  ;[1 1 1] Move Multiplier
  (:Pressed
    (Variables|Default|SetFastMoveMultiplier 2.0))
  (:Released
    (Variables|Default|SetFastMoveMultiplier 1.0)))

(event Input|MouseEvents|LeftMouseButton
  (params (Key :type Key%20Structure :default "None"))
  (bind _selectableobjects (Variables|Default|GetSelectableObjects))
  (bind _hitresult (Class|PlayerController|GetHitResultUnderCursorforObjects _selectableobjects true))
  (bind _hitactor (Collision|BreakHitResult _hitresult))
  ;[1 1 1] Left Mouse Button
  (:Pressed
    (if (Variables|Default|GetbBuildModeActive)
      (if (CallFunction|CanPlaceConstruction)
        (bind _constructionstruct (Default|GetConstructionStruct (Variables|References|GetGhostBuildingRef)))
        (Default|QueueConstruction (Variables|References|GetConstructionManagerRef) _constructionstruct)
        (Default|KillGhost (Variables|References|GetGhostBuildingRef)))
      (else
        (Utilities|IsValid _hitactor
          (:Is%20Valid
            (Default|CallHudRequest _hitactor)))))))

(fn ConstructionScript)

(fn MovementSpeedCalculation
  (return (Math|Float|Clamp(Float) (/ (Variables|/Script/Engine.SpringArmComponent|GetTargetArmLength (Variables|/Game/Blueprints/Framework/BP_CameraPawn.BP_CameraPawn_C|GetSpringArm (Variables|References|GetCameraPawnRef))) 1e+02) 5.0 2e+01)))

(fn SetSightDistance
  (return (+ (Variables|Default|GetSightDistance) (Variables|/Script/Engine.SpringArmComponent|GetTargetArmLength (Variables|/Game/Blueprints/Framework/BP_CameraPawn.BP_CameraPawn_C|GetSpringArm (Variables|References|GetCameraPawnRef))))))

(fn GetSnappedRotationYawAngle
  (bind _camerapawnref (Variables|References|GetCameraPawnRef))
  (bind _buildingrotationrate (Variables|Default|GetBuildingRotationRate))
  (bind _buildingrotationrate_2 (Variables|Default|GetBuildingRotationRate))
  (bind _sphere (Variables|/Game/Blueprints/Framework/BP_CameraPawn.BP_CameraPawn_C|GetSphere _camerapawnref))
  (bind _returnvalue (Transformation|GetWorldRotation _sphere))
  (LocalVariables|SetLYaw (.yaw _returnvalue))
  (if (and (< (.yaw _returnvalue) _buildingrotationrate) (> (.yaw _returnvalue) (* _buildingrotationrate -1.0)))
    (return 0.0)
    (else
      (return (* (.ReturnValue (Math|Float|Division(WholeandRemainder) (Math|Conversions|ToFloat(Integer) (Math|Float|Round (LocalVariables|GetLYaw))) _buildingrotationrate_2)) _buildingrotationrate_2)))))

(fn CanPlaceConstruction
  (return (and (Variables|Default|GetbBuildModeActive) (not (Default|GetIsOverlapping (Variables|References|GetGhostBuildingRef))))))

(fn SetCalendar
  (params (Date :type Array%20of%20Integers))
  (return false))

(fn SetClock
  (params (Time :type Array%20of%20Integers))
  (return false))