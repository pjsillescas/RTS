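; Game state for a city-building game that runs the in-game clock and calendar and registers buildings.
; Tick advances a clockwork value by a speed-scaled time unit, derives time and date, and pushes both to the main UI.
; Speed changes rescale that unit and broadcast it.
; Buildings are sorted into residential and occupational lists; the job search collects open workplaces but stops, reporting none available, at the first full one.
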(event EventBeginPlay
  (bind _asbp_camera_pawn_controller (Utilities|Casting|CastToBP_CameraPawnController (Game|GetPlayerController 0)))
  (Variables|Default|SetControllerRef _asbp_camera_pawn_controller)
  (Variables|Default|SetClockwork (+ (Math|Conversions|ToFloat(Integer) (Variables|Default|GetHours)) (Math|Conversions|ToFloat(Integer) (Variables|Default|GetMinutes)) (Math|Conversions|ToFloat(Integer) (Variables|Default|GetSeconds))))
  (Variables|Default|SetGameDate (Utilities|Array|MakeArray (Variables|Default|GetDay) (Variables|Default|GetMonth) (Variables|Default|GetYear)))
  (Variables|Default|SetTimeUnit (Variables|Default|GetDefaultGameSpeed)))

(event EventTick
  (params (DeltaSeconds :type Float%20%28single-precision%29))
  (Variables|Default|SetClockwork (.ClockworkOut (CallFunction|SetClockwork DeltaSeconds (Variables|Default|GetTimeUnit) (Variables|Default|GetClockwork))))
  (Variables|Default|SetDayTick (.DayTick (CallFunction|SetClockwork DeltaSeconds (Variables|Default|GetTimeUnit) (Variables|Default|GetClockwork))))
  (CallFunction|Clock)
  (CallFunction|Calendar))

(event EventUpdateGameStateSpeed
  (params (Multiplier :type Float%20%28single-precision%29))
  (bind _output_get (Variables|Default|SetSpeedMultiplier Multiplier))
  (bind _output_get_2 (Variables|Default|SetTimeUnit (* (Variables|Default|GetDefaultGameSpeed) _output_get)))
  (Default|CallUpdateGameSpeed _output_get_2))

(fn ConstructionScript)

(fn Clock
  (bind _clockwork (Variables|Default|GetClockwork))
  (bind _returnvalue (* _clockwork 3.6e+03))
  (bind (_remainder _returnvalue_2) (Math|Float|Division(WholeandRemainder) _returnvalue 6e+01))
  (bind _returnvalue_3 (Math|Conversions|ToFloat(Integer) _returnvalue_2))
  (bind (_remainder_2 _returnvalue_4) (Math|Float|Division(WholeandRemainder) _returnvalue_3 6e+01))
  (Variables|Default|SetSeconds (Math|Float|Floor _remainder))
  (Variables|Default|SetMinutes (Math|Float|Floor _remainder_2))
  (Variables|Default|SetHours (Math|Float|Floor (.Remainder (Math|Float|Division(WholeandRemainder) (Math|Conversions|ToFloat(Integer) _returnvalue_4) 24.0))))
  (bind _output_get (Variables|Default|SetGameTime (Utilities|Array|MakeArray (Variables|Default|GetSeconds) (Variables|Default|GetMinutes) (Variables|Default|GetHours))))
  (Class|BPIHUD|SetClock(Message) (Variables|Default|GetMainUIRef) _output_get))

(fn Calendar
  (bind _output_get (Variables|Default|SetDay (+ (Variables|Default|GetDay) (Variables|Default|GetDayTick))))
  (if (> _output_get (Class|KismetMathLibrary|DaysinMonth (Variables|Default|GetYear) (Variables|Default|GetMonth)))
    (Variables|Default|SetDay 1)
    (Math|Integer|IncrementInt (Variables|Default|GetMonth)
      (:%20%20
        _)))
  (if (> (Variables|Default|GetMonth) 12)
    (Variables|Default|SetMonth 1)
    (Math|Integer|IncrementInt (Variables|Default|GetYear)
      (:%20%20
        _)))
  (bind _output_get_2 (Variables|Default|SetGameDate (Utilities|Array|MakeArray (Variables|Default|GetDay) (Variables|Default|GetMonth) (Variables|Default|GetYear))))
  (Class|BPIHUD|SetCalendar(Message) (Variables|Default|GetMainUIRef) _output_get_2))

(fn SetHud
  (params (HudRef :type BPW%20Main%20UI%20Hud%20Object%20Reference))
  (Variables|Default|SetMainUIRef HudRef))

(fn GetCurrentTimeUnit
  (return (Variables|Default|GetTimeUnit)))

(fn AddBuildingtoGame
  (params (Building :type BP%20Building%20Master%20Object%20Reference))
  (bind _output_get (LocalVariables|SetLBuilding Building))
  (switch Utilities|FlowControl|Switch|SwitchonE_BuildingType (.buildingtype (Variables|/Game/Blueprints/Buildings/BP_BuildingMaster.BP_BuildingMaster_C|GetBuildingStruct _output_get))
    (:NewEnumerator0
      (Utilities|Array|AddUnique (Variables|Default|GetResidentialBuildings) (LocalVariables|GetLBuilding)))
    (:NewEnumerator1
      (Utilities|Array|AddUnique (Variables|Default|GetOccupationalBuildings) (LocalVariables|GetLBuilding) :!label _label))
    (:NewEnumerator2
      (goto _label)))
  (return))

(fn GetAvailableJobs
  (if (> (Utilities|Array|Length (Variables|Default|GetOccupationalBuildings)) 0)
    (for _array_element (Variables|Default|GetOccupationalBuildings)
      (bind _output_get (LocalVariables|SetLCurrentBuilding _array_element))
      (if (>= (.NumberOfEmployees (Default|GetEmployees _output_get)) (.maxemployees (Variables|/Game/Blueprints/Buildings/BP_BuildingMaster.BP_BuildingMaster_C|GetBuildingStruct (LocalVariables|GetLCurrentBuilding))))
        (return false (LocalVariables|GetLAvailableJobLocations))
        (else
          (Utilities|Array|AddUnique (LocalVariables|GetLAvailableJobLocations) (LocalVariables|GetLCurrentBuilding)))))
    (return (> (Utilities|Array|Length (LocalVariables|GetLAvailableJobLocations)) 0) (LocalVariables|GetLAvailableJobLocations))
    (else
      (return false (LocalVariables|GetLAvailableJobLocations)))))

(fn SetCalendar
  (params (Date :type Array%20of%20Integers))
  (return false))

(fn SetClock
  (params (Time :type Array%20of%20Integers))
  (return false))