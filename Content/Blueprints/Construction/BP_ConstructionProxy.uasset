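; Placeholder actor for a building under construction, showing its display mesh with a ghost material until the timed work finishes.
; It binds to the game state's game-speed update and keeps a time unit for scaling work.
; Each tick advances a clockwork value into work time spent and compares it to the construction time set from work hours.
; On completion it calls the construction-completed event, then destroys itself after a short delay.
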(event Custom|AdjustTime
  (params (TimeUnit :type Float%20%28single-precision%29))
  (Variables|Default|SetTimeUnit TimeUnit))

(event EventBeginPlay
  (bind _asbp_my_game_state (Utilities|Casting|CastToBP_MyGameState (Game|GetGameState)))
  (bind _output_get (Variables|References|SetGameStateRef _asbp_my_game_state))
  (EventDispatchers|BindEventtoUpdateGameSpeed _output_get (EventDispatchers|CreateEvent :!event Custom|AdjustTime)))

(event Collision|EventActorBeginOverlap
  (params (OtherActor :type Actor%20Object%20Reference)))

(event EventTick
  (params (DeltaSeconds :type Float%20%28single-precision%29))
  (Variables|Default|SetDelta DeltaSeconds)
  (if (not (Variables|Default|GetbIsConstructionCompleted))
    (CallFunction|DoWork)
    (if (>= (Variables|Default|GetWorkTimeSpent) (Variables|Default|GetConstructionTime))
      (Variables|Default|SetbIsConstructionCompleted true)
      (Default|CallConstructionCompleted self)
      (Utilities|FlowControl|Delay 0.2)
      (Actor|DestroyActor))))

(fn ConstructionScript
  (bind _staticmesh (Variables|Default|GetStaticMesh))
  (Components|StaticMesh|SetStaticMesh _staticmesh (Variables|Default|GetDisplayMesh))
  (Rendering|Material|SetMaterial _staticmesh 0 "/Game/Blueprints/Materials/MI_Ghost.MI_Ghost"))

(fn SetConstructionTime
  (params (WorkHours :type Float%20%28single-precision%29))
  (Variables|Default|SetConstructionTime (* WorkHours 6e+01))
  (return))

(fn DoWork
  (bind _output_get (Variables|Default|SetClockwork (.ClockworkOut (CallFunction|SetClockwork (Variables|Default|GetDelta) (Variables|Default|GetTimeUnit) (Variables|Default|GetClockwork)))))
  (Variables|Default|SetWorkTimeSpent (* _output_get 6e+01)))