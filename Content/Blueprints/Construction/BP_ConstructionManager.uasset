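; BP_ConstructionManager is an actor that manages pending building construction, turning placeholder proxies into finished buildings.
; QueueConstruction spawns a proxy with a display mesh at the requested transform, binds to its completion event, and stores proxy and config in index-matched Proxies and Queue arrays.
; On completion, FinishConstruction looks up the config by proxy index, removes both entries, spawns the building class at the stored transform and destroys the proxy.
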(event Custom|BindConstructionComplete
  (params (Proxy :type BP%20Construction%20Proxy%20Object%20Reference))
  (EventDispatchers|BindEventtoConstructionCompleted Proxy (EventDispatchers|CreateEvent :!event Custom|ConstructionCompleted)))

(event Custom|ConstructionCompleted
  (params (Proxy :type BP%20Construction%20Proxy%20Object%20Reference))
  (CallFunction|FinishConstruction Proxy))

(event EventBeginPlay)

(event Collision|EventActorBeginOverlap
  (params (OtherActor :type Actor%20Object%20Reference)))

(event EventTick
  (params (DeltaSeconds :type Float%20%28single-precision%29)))

(fn ConstructionScript)

(fn QueueConstruction
  (params (ConstructionStruct :type S%20Construction%20Structure))
  (bind (_buildingclass _proxyclass _transform _displaymesh) (Utilities|Struct|BreakS_Construction ConstructionStruct))
  (bind _returnvalue (Game|SpawnActorfromClass _proxyclass _transform "AlwaysSpawn" 0 _displaymesh 0))
  (CallFunction|BindConstructionComplete _returnvalue)
  (Utilities|Array|Add (Variables|Default|GetProxies) _returnvalue)
  (Utilities|Array|Add (Variables|Default|GetQueue) ConstructionStruct))

(fn FinishConstruction
  (params (Proxy :type BP%20Construction%20Proxy%20Object%20Reference))
  (bind _output_get (LocalVariables|SetLIndex (Utilities|Array|FindItem (Variables|Default|GetProxies) Proxy)))
  (LocalVariables|SetLConfig (Utilities|Array|Get(acopy) (Variables|Default|GetQueue) _output_get))
  (Utilities|Array|RemoveIndex (Variables|Default|GetQueue) (LocalVariables|GetLIndex))
  (Utilities|Array|RemoveIndex (Variables|Default|GetProxies) (LocalVariables|GetLIndex))
  (Game|SpawnActorfromClass (.BuildingClass (Utilities|Struct|BreakS_Construction (LocalVariables|GetLConfig))) (.Transform (Utilities|Struct|BreakS_Construction (LocalVariables|GetLConfig))) "Undefined" 0 0 0)
  (Actor|DestroyActor Proxy))