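; Master building actor, apparently a base for child buildings, that tracks employees and residents and provides a clickable-style HUD through the camera controller.
; Construction applies the display mesh, entrance and collision box; BeginPlay creates the HUD widget and fills the building struct.
; A HUD request matching this building lerps the camera pawn to it, shows the widget and disables camera navigation and main HUD.
; Hiring respects MaxEmployees, while job assignment, entry, exit and occupant selection are stubs.
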(event Custom|DisplayHud
  (params (Actor :type Actor%20Object%20Reference))
  (bind _buildinghud (Variables|Default|GetBuildingHud))
  (bind _controllerref (Variables|References|GetControllerRef))
  (if (== Actor self)
    (Utilities|FlowControl|Sequence
      (:then_0
        (bind _speed (Timeline|LERPLocationTimeline PlayFromStart)
          (:Update
            (Transformation|SetActorLocation (Variables|/Game/Blueprints/Framework/BP_CameraPawnController.BP_CameraPawnController_C|GetCameraPawnRef (Variables|References|GetControllerRef)) (CallFunction|HudLerpLocation (Transformation|GetActorLocation (Variables|/Game/Blueprints/Framework/BP_CameraPawnController.BP_CameraPawnController_C|GetCameraPawnRef (Variables|References|GetControllerRef))) (Transformation|GetActorLocation) _speed) false false))))
      (:then_1
        (UserInterface|Viewport|AddtoViewport _buildinghud 0)
        (Input|SetInputModeUIOnly _controllerref _buildinghud "DoNotLock")
        (Variables|/Game/Blueprints/Framework/BP_CameraPawnController.BP_CameraPawnController_C|SetbDisableCamNav _controllerref true)
        (Widget|SetIsEnabled (Variables|/Game/Blueprints/Framework/BP_CameraPawnController.BP_CameraPawnController_C|GetMainHudRef _controllerref) false)))))

(event EventBeginPlay
  (bind _output_get (Variables|References|SetControllerRef (.AsBP%20Camera%20Pawn%20Controller (Utilities|Casting|CastToBP_CameraPawnController (Game|GetPlayerController 0)))))
  (EventDispatchers|BindEventtoHudRequest _output_get (EventDispatchers|CreateEvent :!event Custom|DisplayHud))
  (bind _returnvalue (UserInterface|CreateWidget "/Game/Blueprints/HUD/BPW_BuildingHud.BPW_BuildingHud_C" 0 self (Variables|References|GetControllerRef)))
  (Variables|Default|SetBuildingHud _returnvalue)
  (CallFunction|SetBuildingCollisionBox (Variables|Default|GetCollision) (Variables|Default|GetStaticMesh))
  (Utilities|Struct|SetmembersinS_Building (Variables|BuildingInfo|GetBuildingStruct) self))

(event Collision|EventActorBeginOverlap
  (params (OtherActor :type Actor%20Object%20Reference)))

(event EventTick
  (params (DeltaSeconds :type Float%20%28single-precision%29)))

(fn ConstructionScript
  (Components|StaticMesh|SetStaticMesh (Variables|Default|GetStaticMesh) (Variables|Default|GetDisplayMesh))
  (CallFunction|SetBuildingEntrance (Variables|Default|GetEntrance) (Variables|Default|GetStaticMesh))
  (CallFunction|SetBuildingCollisionBox (Variables|Default|GetCollision) (Variables|Default|GetStaticMesh)))

(fn GetEmployees
  (bind _employees (Variables|Default|GetEmployees))
  (bind _returnvalue (Utilities|Array|Length _employees))
  (return (> _returnvalue 0) _returnvalue (Variables|Default|GetEmployees)))

(fn HireEmployee
  (params (NPC :type NPC%20BP%20Object%20Reference))
  (LocalVariables|SetLApplicant NPC)
  (if (< (.NumberOfEmployees (CallFunction|GetEmployees)) (.maxemployees (Variables|BuildingInfo|GetBuildingStruct)))
    (Utilities|Array|AddUnique (Variables|Default|GetEmployees) (LocalVariables|GetLApplicant))
    (return true self)
    (else
      (return false 0))))

(fn AssignEmployeeJob
  (params (Employee :type NPC%20BP%20Object%20Reference))
  (return false 0 "0, 0, 0"))

(fn GetResidents
  (bind _residents (Variables|Default|GetResidents))
  (bind _returnvalue (Utilities|Array|Length _residents))
  (return (> _returnvalue 0) _returnvalue (Variables|Default|GetResidents)))

(fn EnterBuilding
  (params (NPC :type NPC%20BP%20Object%20Reference))
  (return false))

(fn ExitBuilding
  (params (NPC :type NPC%20BP%20Object%20Reference))
  (return false))

(fn GetOccupants
  (bind _list (CallFunction|PickOccupantList))
  (bind _returnvalue (Utilities|Array|Length _list))
  (return (> _returnvalue 0) _returnvalue _list))

(fn PickOccupantList
  (return 0))