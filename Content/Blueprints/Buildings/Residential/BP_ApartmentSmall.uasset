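; BP_ApartmentSmall is a small residential apartment building where NPCs go to sleep.
; EnterBuilding hides the NPC, pauses its AI controller's stamina depletion timer and toggles sleep via SwitchSleep.
; ExitBuilding reveals the NPC, resumes depletion, clears the stamina regain timer and toggles sleep again.
; The event graph is unused, and construction only runs the parent script.
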(event EventBeginPlay)

(event Collision|EventActorBeginOverlap
  (params (OtherActor :type Actor%20Object%20Reference)))

(event EventTick
  (params (DeltaSeconds :type Float%20%28single-precision%29)))

(fn ConstructionScript
  (|CallParentFunction))

(fn EnterBuilding
  (params (NPC :type NPC%20BP%20Object%20Reference))
  (bind _aicontrollerref (Variables|/Game/Blueprints/NPC/NPC_BP.NPC_BP_C|GetAIControllerRef NPC))
  (Rendering|SetActorHiddenInGame NPC true)
  (Utilities|Time|PauseTimerbyHandle (Variables|/Game/Blueprints/NPC/BP_NPCAIController.BP_NPCAIController_C|GetDepleteStaminaHandle _aicontrollerref))
  (Default|SwitchSleep _aicontrollerref)
  (return true))

(fn ExitBuilding
  (params (NPC :type NPC%20BP%20Object%20Reference))
  (bind _aicontrollerref (Variables|/Game/Blueprints/NPC/NPC_BP.NPC_BP_C|GetAIControllerRef NPC))
  (Rendering|SetActorHiddenInGame NPC false)
  (Utilities|Time|UnpauseTimerbyHandle (Variables|/Game/Blueprints/NPC/BP_NPCAIController.BP_NPCAIController_C|GetDepleteStaminaHandle _aicontrollerref))
  (Utilities|Time|ClearandInvalidateTimerbyHandle (Variables|/Game/Blueprints/NPC/BP_NPCAIController.BP_NPCAIController_C|GetRegainStaminaHandle _aicontrollerref))
  (Default|SwitchSleep _aicontrollerref)
  (return true))