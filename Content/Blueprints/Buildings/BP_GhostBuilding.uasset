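; Ghost building actor that previews the selected building during build mode, following the cursor world position snapped to a grid.
; OnSpawn sets the mesh, flags build mode on the controller and opens a Tick gate for movement; KillGhost reverses this.
; ConstructBuilding spawns a temporary building to read its display mesh and construction proxy, restarts the ghost with them, then destroys that actor.
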(event Custom|OnSpawn
  (params (DisplayMesh :type Static%20Mesh%20Object%20Reference) (BuildingClass :type BP%20Building%20Master%20Class%20Reference) (ConstructionProxy :type BP%20Construction%20Proxy%20Class%20Reference))
  (if (not (Variables|Default|GetbActive))
    (Variables|Default|SetDisplayMesh DisplayMesh)
    (Variables|Default|SetBuildingClass BuildingClass)
    (Variables|Default|SetConstructionProxy ConstructionProxy)
    (Variables|Default|SetbActive true)
    (Variables|/Game/Blueprints/Framework/BP_CameraPawnController.BP_CameraPawnController_C|SetbBuildModeActive (Variables|Default|GetControllerRef) true)
    (Components|StaticMesh|SetStaticMesh (Variables|Default|GetGhostBuildingMesh) (Variables|Default|GetDisplayMesh))
    (CallFunction|OpenTickGate)))

(event Custom|KillGhost
  (CallFunction|CloseTickGate)
  (Variables|Default|SetDisplayMesh 0)
  (Variables|Default|SetBuildingClass 0)
  (Variables|Default|SetConstructionProxy 0)
  (Variables|Default|SetbActive false)
  (Components|StaticMesh|SetStaticMesh (Variables|Default|GetGhostBuildingMesh) 0)
  (Variables|/Game/Blueprints/Framework/BP_CameraPawnController.BP_CameraPawnController_C|SetbBuildModeActive (Variables|Default|GetControllerRef) false))

(event Custom|OpenTickGate
  (Utilities|FlowControl|Gate true) ; enters at Open
)

(event Custom|CloseTickGate
  (Utilities|FlowControl|Gate true) ; enters at Close
)

(event EventBeginPlay)

(event Collision|EventActorBeginOverlap
  (params (OtherActor :type Actor%20Object%20Reference)))

(event EventConstructBuilding
  (params (Building :type BP%20Building%20Master%20Class%20Reference))
  (bind _returnvalue (Game|SpawnActorfromClass Building (Math|Transform|MakeTransform "0, 0, 0") "Undefined" 0 (Variables|Default|GetControllerRef) 0))
  (Utilities|FlowControl|Sequence
    (:then_0
      (CallFunction|KillGhost)
      (CallFunction|OnSpawn (Variables|/Game/Blueprints/Buildings/BP_BuildingMaster.BP_BuildingMaster_C|GetDisplayMesh _returnvalue) Building (Variables|/Game/Blueprints/Buildings/BP_BuildingMaster.BP_BuildingMaster_C|GetConstructionProxy _returnvalue)))
    (:then_1
      (Actor|DestroyActor _returnvalue))))

(event EventTick
  (params (DeltaSeconds :type Float%20%28single-precision%29))
  (Utilities|FlowControl|Gate true
    (:Exit
      (Transformation|SetActorLocation (CallFunction|SetGridSnapVector) false false))))

(fn ConstructionScript)

(fn SetGridSnapVector
  (bind _cursorworldposition (Variables|Default|GetCursorWorldPosition))
  (bind _gridsize (Variables|Default|GetGridSize))
  (return (Math|Vector|MakeVector (CallFunction|GridSnap (.x _cursorworldposition) _gridsize) (CallFunction|GridSnap (.y _cursorworldposition) _gridsize) (CallFunction|GridSnap (.z _cursorworldposition) _gridsize))))

(fn SetCalendar
  (params (Date :type Array%20of%20Integers))
  (return false))

(fn SetClock
  (params (Time :type Array%20of%20Integers))
  (return false))