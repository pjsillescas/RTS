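; Construction office building that competes for construction jobs through the controller's Construction Manager, holding one job site at a time.
; A looping timer places a bid whenever the office has employees and no valid current job.
; Winning a bid stores the job site and pauses the timer; the manager's finished-construction event clears the matching site and resumes bidding.
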(event Custom|FinishedConstruction
  (params (JobSite :type BP%20Construction%20Proxy%20Object%20Reference))
  (if (== JobSite (Variables|Default|GetCurrentJobSite))
    (Variables|Default|SetCurrentJobSite 0)
    (Utilities|Time|UnpauseTimerbyHandle (Variables|Default|GetBidTimerHandle))))

(event Custom|BidTimerEvent
  (if (.HasEmployees (CallFunction|GetEmployees))
    (bind _bidsuccessful (CallFunction|BidforJob))
    (if _bidsuccessful
      (Utilities|Time|PauseTimerbyHandle (Variables|Default|GetBidTimerHandle)))))

(event EventBeginPlay
  (|CallParentFunction)
  (bind _output_get (Variables|References|SetConstructionManagerRef (Variables|/Game/Blueprints/Framework/BP_CameraPawnController.BP_CameraPawnController_C|GetConstructionManagerRef (Variables|Default|GetControllerRef))))
  (EventDispatchers|BindEventtoFinishedConstruction _output_get (EventDispatchers|CreateEvent :!event Custom|FinishedConstruction))
  (bind _returnvalue (Utilities|Time|SetTimerbyEvent (EventDispatchers|CreateEvent :!event Custom|BidTimerEvent) 1.0 true))
  (Variables|Default|SetBidTimerHandle _returnvalue))

(event Collision|EventActorBeginOverlap
  (params (OtherActor :type Actor%20Object%20Reference))
  (|CallParentFunction OtherActor) ; This node is disabled and will not be called.\nDrag off pins to build functionality.
)

(event EventTick
  (params (DeltaSeconds :type Float%20%28single-precision%29))
  (|CallParentFunction DeltaSeconds) ; This node is disabled and will not be called.\nDrag off pins to build functionality.
)

(fn ConstructionScript
  (|CallParentFunction))

(fn GetJobStatus
  (return (Utilities|IsValid (Variables|Default|GetCurrentJobSite))))

(fn SetCurrentJob
  (params (JobSite :type BP%20Construction%20Proxy%20Object%20Reference))
  (Variables|Default|SetCurrentJobSite JobSite))

(fn BidforJob
  (if (CallFunction|GetJobStatus)
    (return false)
    (else
      (bind (_jobsite _wonbid) (Default|BidManager (Variables|References|GetConstructionManagerRef) self))
      (LocalVariables|SetLJobSite _jobsite)
      (if _wonbid
        (Variables|Default|SetCurrentJobSite (LocalVariables|GetLJobSite))
        (return true)
        (else
          (return false))))))