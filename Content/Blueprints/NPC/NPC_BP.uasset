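; NPC character Blueprint that gives each spawned NPC a random identity and links it to its AI controller.
; On BeginPlay it picks a random gender, draws a matching name from male or female name enums into its profile, and tints a dynamic body material by gender.
; It caches the NPC AI controller so SetIsBusy can write a busy flag to that controller's Blackboard.
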(event EventBeginPlay
  (CallFunction|GetRandomNPCFeatures)
  (Variables|Default|SetAIControllerRef (.AsBP%20NPCAIController (Utilities|Casting|CastToBP_NPCAIController (AI|GetAIController self)))))

(event Collision|EventActorBeginOverlap
  (params (OtherActor :type Actor%20Object%20Reference)))

(event EventTick
  (params (DeltaSeconds :type Float%20%28single-precision%29)))

(fn ConstructionScript)

(fn GetRandomNPCFeatures
  (bind _returnvalue (Rendering|Material|CreateDynamicMaterialInstance (Variables|Character|GetMesh) 0 "/Game/Mannequin/Character/Materials/MI_Body.MI_Body" "None" :!class /Script/Engine.PrimitiveComponent))
  (LocalVariables|SetLMaterialInstance _returnvalue)
  (bind _output_get (LocalVariables|SetRandomGender (Utilities|Enum|ByteToEnumE_GenderType (Math|Conversions|ToByte(Integer) (Math|Random|RandomIntegerinRange 0 1)))))
  (Variables|Default|SetProfile (Utilities|Struct|MakeS_NPCProfile (CallFunction|GetRandomName _output_get) _output_get))
  (switch Utilities|FlowControl|Switch|SwitchonE_GenderType _output_get
    (:NewEnumerator0
      (Rendering|Material|SetVectorParameterValue (LocalVariables|GetLMaterialInstance) "BodyColor" (LocalVariables|GetMaleColor) :!class /Script/Engine.MaterialInstanceDynamic))
    (:NewEnumerator1
      (Rendering|Material|SetVectorParameterValue (LocalVariables|GetLMaterialInstance) "BodyColor" (LocalVariables|GetFemaleColor) :!class /Script/Engine.MaterialInstanceDynamic))))

(fn GetRandomName
  (params (Gender :type E_GenderType%20Enum :default "NewEnumerator0"))
  (switch Utilities|FlowControl|Switch|SwitchonE_GenderType Gender
    (:NewEnumerator0
      (return (CallFunction|GetRandomMaleName)))
    (:NewEnumerator1
      (return (CallFunction|GetRandomFemaleName)))))

(fn GetRandomMaleName
  (return (Utilities|String|EnumtoString (Utilities|Enum|ByteToEnumE_NameMale (Math|Conversions|ToByte(Integer) (Math|Random|RandomIntegerinRange 0 (- (|GetNumEnumEntries) 1)))))))

(fn GetRandomFemaleName
  (return (Utilities|String|EnumtoString (Utilities|Enum|ByteToEnumE_NameFemale (Math|Conversions|ToByte(Integer) (Math|Random|RandomIntegerinRange 0 (- (|GetNumEnumEntries) 1)))))))

(fn SetIsBusy
  (params (bIsBusy :type Boolean))
  (AI|Components|Blackboard|SetValueasBool (AI|GetBlackboard (Variables|Default|GetAIControllerRef)) (Variables|Default|GetIsBusy) bIsBusy))